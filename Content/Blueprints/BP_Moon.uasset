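; BP_Moon is a moon actor that gets pushed when clicked.
; On BeginPlay it enables click events on the first player controller and hides its static mesh component, leaving child components' visibility untouched.
; A click on that mesh applies a mass-independent impulse in Y and Z, scaled by horizontal and vertical strengths from the offset between actor location and deprojected cursor position.
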(event `self.ReceiveBeginPlay`
  (set `PlayerController.bEnableClickEvents` true (`GameplayStatics.GetPlayerController` 0))
  (`SceneComponent.SetVisibility` (`self.StaticMeshComponent`) false false))

(event `self.StaticMeshComponent.OnClicked`
  (params (TouchedComponent :type "PrimitiveComponent Object Reference") (ButtonPressed :type "Key Structure"))
  (bind (_returnvalue_x _returnvalue_y _returnvalue_z) (`KismetMathLibrary.BreakVector` (`self.K2_GetActorLocation`)))
  (bind _worldlocation (`PlayerController.DeprojectMousePositionToWorld` (`GameplayStatics.GetPlayerController` 0)))
  (`PrimitiveComponent.AddImpulse` TouchedComponent (`KismetMathLibrary.MakeVector` 0.0 (* (`self.HorizontalStrength`) (- _returnvalue_y (.y _worldlocation))) (* (- _returnvalue_z (.z _worldlocation)) (`self.VerticalStrength`))) "None" true))

(fn `UserConstructionScript`)