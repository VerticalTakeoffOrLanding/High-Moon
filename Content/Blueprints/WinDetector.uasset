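; WinDetector is an actor that decides the win or loss of the game from the position of BP_Moon.
; Each Tick it finds the moon and shows the existing win menu widget once its Z reaches WinHeight.
; Otherwise it projects the moon to screen space and shows the existing lose menu widget when it leaves the viewport, allowing a horizontal pixel margin.
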(event `self.ReceiveTick`
  (params (DeltaSeconds :type "Float (single-precision)"))
  (bind (_returnvalue_x _returnvalue_y) (`KismetMathLibrary.BreakVector2D` (`WidgetLayoutLibrary.GetViewportSize`)))
  (bind _returnvalue (`GameplayStatics.GetActorOfClass` "/Game/Blueprints/BP_Moon.BP_Moon_C"))
  (if (>= (.z (.location (`self.GetTransform` _returnvalue))) (`self.WinHeight`))
    (bind _foundwidgets (`WidgetBlueprintLibrary.GetAllWidgetsOfClass` "/Game/Blueprints/Widgets/WinMenuWidget.WinMenuWidget_C" false))
    (`UserWidget.AddToViewport` (select `int` 0 :`0` _foundwidgets :`1` _) 0)
    (else
      (bind _screenlocation (`PlayerController.ProjectWorldLocationToScreen` (`GameplayStatics.GetPlayerController` 0) (`self.K2_GetActorLocation` _returnvalue) false))
      (if (not (and (> (+ 50.0 (`KismetMathLibrary.BreakVector2D` _screenlocation)) 0.0) (< (- (`KismetMathLibrary.BreakVector2D` _screenlocation) 50.0) _returnvalue_x) (> (`.Y` (`KismetMathLibrary.BreakVector2D` _screenlocation)) 0.0) (< (`.Y` (`KismetMathLibrary.BreakVector2D` _screenlocation)) _returnvalue_y)))
        (bind _foundwidgets_2 (`WidgetBlueprintLibrary.GetAllWidgetsOfClass` "/Game/Blueprints/Widgets/LoseMenuWidget.LoseMenuWidget_C" false))
        (`UserWidget.AddToViewport` (select `int` 0 :`0` _foundwidgets_2 :`1` _) 0)))))

(fn `UserConstructionScript`)